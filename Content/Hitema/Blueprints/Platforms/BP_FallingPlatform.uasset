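; A falling platform that drops when the player touches it, then respawns at its starting transform.
; When BP_Player overlaps the Box, it plays a sound and runs the RotateCrate timeline, which drives the mesh's pitch as a cue before the fall.
; When the timeline finishes, the mesh simulates physics for a few seconds, then physics turns off and it teleports back to the transform cached at BeginPlay.
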(event OnComponentBeginOverlap(Box)
  (params (OverlappedComponent :type Primitive%20Component%20Object%20Reference) (OtherActor :type Actor%20Object%20Reference) (OtherComp :type Primitive%20Component%20Object%20Reference) (OtherBodyIndex :type Integer) (bFromSweep :type Boolean) (SweepResult :type Hit%20Result%20Structure%20%28by%20ref%29))
  (bind _asbp_player (Utilities|Casting|CastToBP_Player OtherActor))
  (Variables|Default|SetPlayerReference _asbp_player)
  (Audio|PlaySound2D "/Engine/EditorSounds/Notifications/CompileFailed_Cue.CompileFailed_Cue" 1.0 1.0 0.0 0 0)
  (bind _rotatevalue (Timeline|RotateCrate PlayFromStart)
    (:Update
      (Transformation|SetWorldRotation (Variables|Default|GetMesh) (Math|Rotator|MakeRotator 0.0 _rotatevalue 0.0) false false))
    (:Finished
      (Physics|SetSimulatePhysics (Variables|Default|GetMesh) true)
      (Utilities|FlowControl|Delay 5.0)
      (Physics|SetSimulatePhysics (Variables|Default|GetMesh) false)
      (Transformation|SetWorldTransform (Variables|Default|GetMesh) (Variables|Default|GetDefaultRespawnTransform) false true))))

(event EventBeginPlay
  (Variables|Default|SetDefaultRespawnTransform (Transformation|GetWorldTransform (Variables|Default|GetMesh))))

(fn ConstructionScript)