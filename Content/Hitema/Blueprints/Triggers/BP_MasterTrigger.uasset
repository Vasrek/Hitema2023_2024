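; Configurable box trigger volume that acts as either a death zone or a checkpoint when the player overlaps it, chosen by TriggerType.
; Death calls the player's Death function.
; Checkpoint fires once, passes the Arrow's transform to the player as a new respawn point, and plays a sound, a healing Niagara effect, and a delayed repeat sound.
; The construction script sizes the box from BoxScale.
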(event OnComponentBeginOverlap(Box)
  (params (OverlappedComponent :type Primitive%20Component%20Object%20Reference) (OtherActor :type Actor%20Object%20Reference) (OtherComp :type Primitive%20Component%20Object%20Reference) (OtherBodyIndex :type Integer) (bFromSweep :type Boolean) (SweepResult :type Hit%20Result%20Structure%20%28by%20ref%29))
  (bind _asbp_player (Utilities|Casting|CastToBP_Player OtherActor))
  (Variables|Default|SetPlayerReference _asbp_player)
  (switch Utilities|FlowControl|Switch|SwitchonE_TriggersType (Variables|BoxSettings|GetTriggerType)
    (:NewEnumerator0
      (Default|Death (Variables|Default|GetPlayerReference)))
    (:NewEnumerator1
      (if (Variables|Default|GetCanBeActivated?)
        (Variables|Default|SetCanBeActivated? false)
        (Default|AddNewRespawnTransform (Variables|Default|GetPlayerReference) (Transformation|GetWorldTransform (Variables|Default|GetArrow)))
        (Audio|PlaySound2D "/Engine/EditorSounds/Notifications/CompileSuccess.CompileSuccess" 1.0 1.0 0.0 0 0)
        (Niagara|SpawnSystemAttached "/Game/sA_PickupSet_1/Fx/NiagaraSystems/NS_Healing_2.NS_Healing_2" (Variables|/Script/Engine.Character|GetMesh (Variables|Default|GetPlayerReference)) "None" "0.000000,0.000000,100.000000" "0, 0, 0" "KeepRelativeOffset" false)
        (Utilities|FlowControl|Delay 1.0)
        (Audio|PlaySound2D "/Engine/EditorSounds/Notifications/CompileSuccess.CompileSuccess" 1.0 1.0 0.0 0 0)))))

(fn ConstructionScript
  (Components|Box|SetBoxExtent (Variables|Default|GetBox) (Variables|BoxSettings|GetBoxScale) true))